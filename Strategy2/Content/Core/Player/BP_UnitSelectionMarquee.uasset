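; Drag-selection marquee actor that selects friendly units through a collision box in the world.
; While resizing, Tick stretches the box between the actor's location and the cursor trace hit, and updates the HUD widget's marquee.
; Overlaps message the player controller to select Friendly Selection_Event actors or deselect those leaving mid-drag.
; Start/End functions toggle resizing, query collision and the HUD marquee, so ending the drag keeps the selection.
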(event OnComponentBeginOverlap(BoxCol)
  (params (OverlappedComponent :type Primitive%20Component%20Object%20Reference) (OtherActor :type Actor%20Object%20Reference) (OtherComp :type Primitive%20Component%20Object%20Reference) (OtherBodyIndex :type Integer) (bFromSweep :type Boolean) (SweepResult :type Hit%20Result%20Structure%20%28by%20ref%29))
  (if (Utilities|DoesObjectImplementInterface OtherActor "/Game/Core/Building/Selection_Event.Selection_Event_C")
    (bind _teamattitude (Class|SelectionEvent|GetTeamAttitude(Message) OtherActor))
    (if (Utilities|Enum|Equal(Enum) _teamattitude "Friendly")
      (Class|SelectionEvent|SelectThisActor(Message) (Game|GetPlayerController 0) OtherActor))))

(event OnComponentEndOverlap(BoxCol)
  (params (OverlappedComponent :type Primitive%20Component%20Object%20Reference) (OtherActor :type Actor%20Object%20Reference) (OtherComp :type Primitive%20Component%20Object%20Reference) (OtherBodyIndex :type Integer))
  (if (and (Variables|Default|GetShoodResizeMarqee) (Utilities|DoesObjectImplementInterface OtherActor "/Game/Core/Building/Selection_Event.Selection_Event_C"))
    (Class|SelectionEvent|DeselectThisActor(Message) (Game|GetPlayerController 0) OtherActor)))

(event EventBeginPlay)

(event Collision|EventActorBeginOverlap
  (params (OtherActor :type Actor%20Object%20Reference)))

(event EventTick
  (params (DeltaSeconds :type Float%20%28single-precision%29))
  (if (Variables|Default|GetShoodResizeMarqee)
    (bind _asplayer_control (Utilities|Casting|CastToPlayerControl (Game|GetPlayerController 0)))
    (Variables|Default|SetEndMouseLocation (.Location (Collision|BreakHitResult (.HitResult (Game|Player|GetHitResultUnderCursorbyChannel _asplayer_control "TraceTypeQuery1" true)))))
    (Transformation|SetWorldLocation (Variables|Default|GetBoxCol) (Math|Vector|Lerp(Vector) (Transformation|GetActorLocation) (Variables|Default|GetEndMouseLocation) 0.5) false false)
    (Components|Box|SetBoxExtent (Variables|Default|GetBoxCol) (Math|Vector|MakeVector (.x (/ (Math|Vector|VectorGetAbs (- (Transformation|GetActorLocation) (Variables|Default|GetEndMouseLocation))) 2.0)) (.y (/ (Math|Vector|VectorGetAbs (- (Transformation|GetActorLocation) (Variables|Default|GetEndMouseLocation))) 2.0)) 3e+02) true)
    (bind _asbp_hud (Utilities|Casting|CastToBP_Hud (HUD|GetHUD (Game|GetPlayerController 0))))
    (Default|UpdateMarquee (Variables|/Game/Core/Player/BP_Hud.BP_Hud_C|GetHudWidgetRef _asbp_hud))))

(fn ConstructionScript)

(fn StartResuzingMarquee
  (Variables|Default|SetShoodResizeMarqee true)
  (Collision|SetCollisionEnabled (Variables|Default|GetBoxCol) "QueryOnly")
  (bind _asbp_hud (Utilities|Casting|CastToBP_Hud (HUD|GetHUD (Game|GetPlayerController 0))))
  (Default|StartMarqueeUpdate (Variables|/Game/Core/Player/BP_Hud.BP_Hud_C|GetHudWidgetRef _asbp_hud)))

(fn EndResuzingMarquee
  (Variables|Default|SetShoodResizeMarqee false)
  (Collision|SetCollisionEnabled (Variables|Default|GetBoxCol) "NoCollision")
  (bind _asbp_hud (Utilities|Casting|CastToBP_Hud (HUD|GetHUD (Game|GetPlayerController 0))))
  (Default|StopMarqueeUpdate (Variables|/Game/Core/Player/BP_Hud.BP_Hud_C|GetHudWidgetRef _asbp_hud)))